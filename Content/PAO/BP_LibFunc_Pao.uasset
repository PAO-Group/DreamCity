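; Blueprint function library of shared helpers for procedural mesh and spline construction, plus line-trace hit tests from controller view or input rays.
; Mesh helpers derive transforms from bounds and target sizes, then add components or instances, reusing instanced components per mesh and overlay material.
; Scale can feed materials through dynamic parameters or per-instance custom data for UVs.
; Other helpers turn polygons with holes into linear splines and resolve referenced numeric values.
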(fn GetForwardPos
  (params (OriginPos :type Vector) (Dicection :type Rotator) (Length :type Float%20%28double-precision%29))
  (return (+ OriginPos (* (Math|Vector|GetForwardVector Dicection) Length))))

(fn GetSideTransform
  (params (FrameSide :type ST%20Frame%20Side%20Structure) (SideType :type E_SizeType%20Enum :default "NewEnumerator5") (OriginSize :type Float%20%28double-precision%29) (Revert :type Boolean))
  (return (Utilities|Select :Index SideType :NewEnumerator5 (* (- (.size FrameSide) (.bordernear FrameSide)) -0.5) :NewEnumerator9 (* (- (.size FrameSide) (.borderfar FrameSide)) 0.5) :NewEnumerator6 (/ (- (.bordernear FrameSide) (.borderfar FrameSide)) 2.0) :NewEnumerator7 0.0) (Utilities|Operators|Divide (Utilities|Select :Index SideType :NewEnumerator5 (.bordernear FrameSide) :NewEnumerator9 (.borderfar FrameSide) :NewEnumerator6 (Utilities|Operators|Subtract (.size FrameSide) (.bordernear FrameSide) (.borderfar FrameSide)) :NewEnumerator7 (.size FrameSide)) OriginSize (select Revert -1.0 1.0))))

(fn SetFrameTransform
  (params (MeshComponent :type Static%20Mesh%20Component%20Object%20Reference) (XSide :type ST%20Frame%20Side%20Structure) (YSide :type ST%20Frame%20Side%20Structure) (ZSide :type ST%20Frame%20Side%20Structure) (XSideType :type E_SizeType%20Enum :default "NewEnumerator5") (YSideType :type E_SizeType%20Enum :default "NewEnumerator5") (ZSideType :type E_SizeType%20Enum :default "NewEnumerator5") (XRevert :type Boolean) (YRevert :type Boolean) (ZRevert :type Boolean))
  (bind (_min _max) (Components|StaticMesh|GetLocalBounds MeshComponent))
  (Utilities|FlowControl|Sequence
    (:then_0
      ;[0.15 0.15 0.15 0.5] 获取尺寸
      (LocalVariables|SetOriginSize (- _max _min)))
    (:then_1
      (bind (_location _scale) (Frame|GetSideTransform XSide XSideType (.x (LocalVariables|GetOriginSize)) XRevert))
      (bind (_location_2 _scale_2) (Frame|GetSideTransform YSide YSideType (.y (LocalVariables|GetOriginSize)) YRevert))
      (bind (_location_3 _scale_3) (Frame|GetSideTransform ZSide ZSideType (.z (LocalVariables|GetOriginSize)) ZRevert))
      (Transformation|SetRelativeTransform MeshComponent (Math|Transform|MakeTransform (Math|Vector|MakeVector _location _location_2 _location_3) "0, 0, 0" (Math|Vector|MakeVector _scale _scale_2 _scale_3)) false false))))

(fn HitTestbyControllerViewPoint
  (params (控制器 :type Controller%20Object%20Reference) (视线范围 :type Float%20%28double-precision%29) (bTraceComplex :type Boolean) (ActorsToIgnore :type Array%20of%20Actor%20Object%20References) (TraceChannel :type ETraceTypeQuery%20Enum :default "TraceTypeQuery1") (DrawDebugType :type EDrawDebugTrace%20Enum :default "None") (TraceColor :type Linear%20Color%20Structure :default "(R=0.706958,G=0.000000,B=1.000000,A=1.000000)") (TraceHitColor :type Linear%20Color%20Structure :default "(R=0.000000,G=0.000000,B=0.000000,A=1.000000)") (DrawTime :type Float%20%28single-precision%29))
  (bind (_location _rotation) (Pawn|GetPlayerViewPoint 控制器))
  (bind (_outhit _returnvalue) (Collision|LineTraceByChannel 0 _location (+ _location (* _rotation 视线范围)) TraceChannel bTraceComplex ActorsToIgnore DrawDebugType true TraceColor TraceHitColor DrawTime))
  (return _outhit _returnvalue))

(fn HitTestbyInputDeviceRay
  (params (InputDeviceRay :type Input%20Device%20Ray%20Structure%20%28by%20ref%29) (ActorsToIgnore :type Array%20of%20Actor%20Object%20References))
  (bind _worldray (Utilities|Struct|BreakInputDeviceRay InputDeviceRay))
  (bind (_outhit _returnvalue) (Collision|LineTraceByChannel 0 (.origin _worldray) (+ (.origin _worldray) (* (.direction _worldray) (LocalVariables|GetHitDistance))) "TraceTypeQuery1" false ActorsToIgnore "ForOneFrame"))
  (return _outhit _returnvalue))

(fn GetorSetMaterial
  (params (MeshComponent :type Mesh%20Component%20Object%20Reference) (Material :type Material%20Interface%20Object%20Reference))
  (bind _returnvalue (Rendering|Material|GetMaterials MeshComponent))
  (bind _returnvalue_2 (Utilities|Array|FindItem _returnvalue Material))
  (if (== _returnvalue_2 -1)
    ;[0.15 0.15 0.15 0.5] 找不到材质，创建新材质
    (bind _output_get (LocalVariables|SetNewIndex (Utilities|Array|Length _returnvalue)))
    (Rendering|Material|SetMaterial MeshComponent _output_get Material)
    (return (LocalVariables|GetNewIndex))
    (else
      (return _returnvalue_2))))

(fn GetorSetInstancedStaticMeshComponent
  (params (Actor :type Actor%20Object%20Reference) (StaticMesh :type Static%20Mesh%20Object%20Reference) (Material :type Material%20Object%20Reference))
  (for _array_element (Actor|GetComponentsByClass Actor "/Script/Engine.InstancedStaticMeshComponent")
    (if (and (== (Variables|/Script/Engine.StaticMeshComponent|GetStaticMesh _array_element) StaticMesh) (== (Rendering|Material|GetOverlayMaterial _array_element :!class /Script/Engine.MeshComponent) Material))
      (return _array_element)))
  ;[0.15 0.15 0.15 0.5] 如果未找到指定StaticMesh则创建新的InstancedStaticMeshComponent
  (bind _returnvalue (Game|AddComponentbyClass Actor "/Script/Engine.InstancedStaticMeshComponent" false))
  (Components|StaticMesh|SetStaticMesh _returnvalue StaticMesh)
  (Rendering|Material|SetOverlayMaterial _returnvalue Material :!class /Script/Engine.MeshComponent)
  (return _returnvalue))

(fn LimitRange
  (params (Value :type Float%20%28double-precision%29) (MinValue :type Float%20%28double-precision%29) (MaxValue :type Float%20%28double-precision%29))
  (return (Math|Float|Min(Float) (Math|Float|Max(Float) Value MinValue) MaxValue)))

(fn AddStaticMeshInstance
  (params (InstancedMeshComponent :type Instanced%20Static%20Mesh%20Component%20Object%20Reference) (InstanceTransform :type Transform%20%28by%20ref%29) (CustomDataValues :type Array%20of%20Floats%20%28single-precision%29))
  (bind _returnvalue (Components|InstancedStaticMesh|AddInstance InstancedMeshComponent InstanceTransform false))
  (Class|InstancedStaticMeshComponent|SetNumCustomDataFloats InstancedMeshComponent (Utilities|Array|Length CustomDataValues))
  (for (_array_element _array_index) CustomDataValues
    (Components|InstancedStaticMesh|SetCustomDataValue InstancedMeshComponent _returnvalue _array_index _array_element false)))

(fn AddStaticMeshInstancebyPos
  (params (Actor :type Actor%20Object%20Reference) (StaticMesh :type Static%20Mesh%20Object%20Reference) (StartPos :type Vector :default "0, 0, 0") (Direction :type Rotator :default "0, 0, 0") (Size :type Vector :default "0, 0, 0") (AutoSize :type Boolean) (CustomDataValues :type Array%20of%20Floats%20%28single-precision%29))
  (bind (_transform _targetpos _targetsize) (Geometry|CalcStaticMeshTransform StaticMesh StartPos Direction Size AutoSize))
  ;[0.15 0.15 0.15 0.5] 添加InstancedStaticMesh组件
  (bind _instancedstaticmeshcomponent (Geometry|GetorSetInstancedStaticMeshComponent Actor StaticMesh))
  ;[0.15 0.15 0.15 0.5] 计算尺寸并添加实例
  (Geometry|AddStaticMeshInstance _instancedstaticmeshcomponent _transform CustomDataValues)
  (return _targetpos _targetsize))

(fn GetUpPos
  (params (OriginPos :type Vector) (Dicection :type Rotator) (Length :type Float%20%28double-precision%29))
  (return (+ OriginPos (* (Math|Vector|GetUpVector Dicection) Length))))

(fn GetRightPos
  (params (OriginPos :type Vector) (Dicection :type Rotator) (Length :type Float%20%28double-precision%29))
  (return (+ OriginPos (* (Math|Vector|GetRightVector Dicection) Length))))

(fn AddStaticMeshbyPos
  (params (Actor :type Actor%20Object%20Reference) (StaticMesh :type Static%20Mesh%20Object%20Reference) (StartPos :type Vector :default "0, 0, 0") (Direction :type Rotator :default "0, 0, 0") (Size :type Vector :default "0, 0, 0") (AutoSize :type Boolean))
  (bind (_transform _targetpos _targetsize) (Geometry|CalcStaticMeshTransform StaticMesh StartPos Direction Size AutoSize))
  (LocalVariables|SetUScale (.x (.Scale (Math|Transform|BreakTransform _transform))))
  (LocalVariables|SetVScale (.z (.Scale (Math|Transform|BreakTransform _transform))))
  (bind _returnvalue (Game|AddComponentbyClass Actor "/Script/Engine.StaticMeshComponent" false _transform))
  (bind _output_get (LocalVariables|SetNewComponent _returnvalue))
  (Components|StaticMesh|SetStaticMesh _output_get StaticMesh)
  (for (_array_element _array_index) (Rendering|Material|GetMaterials _output_get)
    (bind _returnvalue_2 (Rendering|Material|CreateDynamicMaterialInstance _output_get _array_element "None" "Transient" :!class /Script/Engine.KismetMaterialLibrary))
    (Rendering|Material|SetScalarParameterValue _returnvalue_2 "UScale" (LocalVariables|GetUScale) :!class /Script/Engine.MaterialInstanceDynamic)
    (Rendering|Material|SetScalarParameterValue _returnvalue_2 "VScale" (LocalVariables|GetVScale) :!class /Script/Engine.MaterialInstanceDynamic)
    (Rendering|Material|SetMaterial (LocalVariables|GetNewComponent) _array_index _returnvalue_2))
  (return _targetpos _targetsize))

(fn CalcStaticMeshTransform
  (params (StaticMesh :type Static%20Mesh%20Object%20Reference) (StartPos :type Vector) (Direcction :type Rotator) (Size :type Vector) (AutoSize :type Boolean))
  (bind _returnvalue (StaticMesh|GetBoundingBox StaticMesh))
  (bind (_transform _targetpos _targetsize) (Geometry|CalcTransformbyPos StartPos Direcction (- (.max _returnvalue) (.min _returnvalue)) Size AutoSize))
  (return _transform _targetpos _targetsize))

(fn CalcTransformbyPos
  (params (StartPos :type Vector) (Direcction :type Rotator) (OriginSize :type Vector) (Size :type Vector) (AutoSize :type Boolean))
  (bind _returnvalue (select AutoSize OriginSize Size))
  ;[0.15 0.15 0.15 0.5] 获取目标位置
  (bind _targetpos (Math|GetForwardPos StartPos Direcction (.X (Math|Vector|BreakVector _returnvalue))))
  (return (Math|Transform|MakeTransform StartPos Direcction (select AutoSize "1.000000,1.000000,1.000000" (/ Size OriginSize))) _targetpos _returnvalue))

(fn GetStaticMeshOriginSize
  (params (StaticMesh :type Static%20Mesh%20Object%20Reference))
  (bind _returnvalue (StaticMesh|GetBoundingBox StaticMesh))
  (return (- (.max _returnvalue) (.min _returnvalue))))

(fn CalcStaticMeshScale
  (params (StaticMesh :type Static%20Mesh%20Object%20Reference) (TargetSize :type Vector))
  (bind _originsize (Geometry|GetStaticMeshOriginSize StaticMesh))
  (return (/ TargetSize (Math|Vector|MakeVector (select (<= (.x _originsize) 0.0001) 1.0 (.x _originsize)) (select (<= (.y _originsize) 0.0001) 1.0 (.y _originsize)) (select (<= (.z _originsize) 0.0001) 1.0 (.z _originsize))))))

(fn AddStaticMeshInstancewithScale
  (params (InstancedStaticMeshComponent :type Instanced%20Static%20Mesh%20Component%20Object%20Reference) (Transform :type Transform%20%28by%20ref%29) (TargetSize :type Vector) (UVScale :type Boolean))
  (bind _staticmesh (Variables|/Script/Engine.StaticMeshComponent|GetStaticMesh InstancedStaticMeshComponent))
  (bind _scale (Geometry|CalcStaticMeshScale _staticmesh TargetSize))
  (bind (_x _y) (Math|Vector|BreakVector _scale))
  (Geometry|AddStaticMeshInstance InstancedStaticMeshComponent (Math|Transform|ComposeTransforms (Math|Transform|MakeTransform "0, 0, 0" "0, 0, 0" _scale) Transform) (select UVScale (Utilities|Array|MakeArray _x _y) 0)))

(fn CalcCornerQuadrangle
  (params (Y1 :type Float%20%28double-precision%29) (Y2 :type Float%20%28double-precision%29) (Angle :type Float%20%28double-precision%29))
  (bind _returnvalue (Math|Trig|Cos(Degrees) Angle))
  (bind _returnvalue_2 (* Y1 Y2))
  (bind _returnvalue_3 (- 1.0 _returnvalue_2))
  (bind _returnvalue_4 (/ _returnvalue_3 _returnvalue))
  (return (Math|Float|Sqrt (- _returnvalue_4 (* Y1 Y1))) (Math|Float|Sqrt (- _returnvalue_4 (* Y2 Y2)))))

(fn SetSplinePointsType
  (params (SplineComponent :type Spline%20Component%20Object%20Reference) (PointType :type ESplinePointType%20Enum :default "Linear"))
  (for _index (range 0 (- (Spline|GetNumberOfSplinePoints SplineComponent) 1))
    (Spline|SetSplinePointType SplineComponent _index PointType true))
  (Spline|UpdateSpline SplineComponent))

(fn AddSplinebyPolyline
  (params (Actor :type Actor%20Object%20Reference) (Points :type Array%20of%20Vector%202D%20Structures) (IsClosed :type Boolean) (Transform :type Transform) (Tags :type Array%20of%20Names))
  (bind _returnvalue (Game|AddComponentbyClass Actor "/Script/Engine.SplineComponent" false Transform))
  (Spline|ClearSplinePoints _returnvalue true)
  (Polygon|SetSplinebyPolyline _returnvalue Points IsClosed)
  (Variables|/Script/Engine.ActorComponent|SetComponentTags _returnvalue Tags))

(fn AddSplinebyPolygonList
  (params (Actor :type Actor%20Object%20Reference) (PolygonList :type Geometry%20Script%20General%20Polygon%20List%20Structure) (Transform :type Transform))
  (bind _polylines (Polygon|PolygonListtoPolylines PolygonList))
  (Polygon|AddSplinebyPolylines Actor _polylines Transform))

(fn AddSplinebyPolylines
  (params (Actor :type Actor%20Object%20Reference) (PolygonList :type Array%20of%20ST%20Path%20Structures) (Transform :type Transform) (Tags :type Array%20of%20Names))
  (for _array_element PolygonList
    (Polygon|AddSplinebyPolyline Actor (.points _array_element) (.closed _array_element) Transform Tags)))

(fn PolygonListtoPolylines
  (params (PolygonList :type Geometry%20Script%20General%20Polygon%20List%20Structure))
  (LocalVariables|SetNewPolylines (Utilities|Array|MakeArray))
  (bind _returnvalue (Class|GeometryScriptLibraryPolygonListFunctions|GetPolygonCount PolygonList))
  (for _index (range 0 (- _returnvalue 1))
    ;[0.15 0.15 0.15 0.5] 处理每一个多边形
    (bind _returnvalue_2 (Class|GeometryScriptLibraryPolygonListFunctions|GetPolygonHoleCount PolygonList _index))
    (for _index_2 (range -1 (- _returnvalue_2 1))
      ;;[0.15 0.15 0.15 0.5] 处理每一个洞
      (bind _outvertices (Class|GeometryScriptLibraryPolygonListFunctions|GetPolygonVertices PolygonList _index _index_2))
      (Utilities|Array|Add (LocalVariables|GetNewPolylines) (Utilities|Struct|MakeST_Path _outvertices true))))
  (return (LocalVariables|GetNewPolylines)))

(fn SetSplinebyPolyline
  (params (SplineComponent :type Spline%20Component%20Object%20Reference) (Points :type Array%20of%20Vector%202D%20Structures) (IsClosed :type Boolean))
  (Variables|/Script/Engine.SplineComponent|SetbInputSplinePointsToConstructionScript SplineComponent true)
  (Spline|SetClosedLoop SplineComponent IsClosed true)
  (for _array_element Points
    (Spline|AddSplinePoint SplineComponent (Math|Conversions|ToVector(Vector2D) _array_element) "Local" true))
  (Polygon|SetSplinePointsType SplineComponent "Linear"))

(fn GetNumberbyRef
  (params (NumberMap :type I%20Number%20Map%20Interface) (Ref :type Name) (Value :type Float%20%28double-precision%29))
  (bind (_numbermap _valid) (Default|GetNumberbyRef NumberMap Ref))
  (return (+ (select _valid _numbermap 0.0) Value)))

(fn GetVectorsbyRef
  (params (NumberMap :type I%20Number%20Map%20Interface) (VectorRefs :type Array%20of%20ST%20Vector%20Ref%20Structures))
  (LocalVariables|SetNewArray (Utilities|Array|MakeArray))
  (for _array_element VectorRefs
    (bind _targetvalue (NumberRef|GetNumberbyRef NumberMap (.xref _array_element) (.x _array_element)))
    (bind _targetvalue_2 (NumberRef|GetNumberbyRef NumberMap (.yref _array_element) (.y _array_element)))
    (Utilities|Array|Add (LocalVariables|GetNewArray) (Math|Vector2D|MakeVector2D _targetvalue _targetvalue_2)))
  (return (LocalVariables|GetNewArray)))

(fn CalcMeshSizebyMode
  (params (XSizeMode :type PAO_E_MeshSizeMode%20Enum :default "NewEnumerator0") (YSizeMode :type PAO_E_MeshSizeMode%20Enum :default "NewEnumerator0") (ZSizeMode :type PAO_E_MeshSizeMode%20Enum :default "NewEnumerator0") (OriginSize :type Vector) (FixedSize :type Vector) (SprintSize :type Vector))
  (bind (_x _y _z) (Math|Vector|BreakVector OriginSize))
  (bind (_x_2 _y_2 _z_2) (Math|Vector|BreakVector FixedSize))
  (bind (_x_3 _y_3 _z_3) (Math|Vector|BreakVector SprintSize))
  (return (Math|Vector|MakeVector (Utilities|Select :Index XSizeMode :NewEnumerator0 _x :NewEnumerator1 _x_2 :NewEnumerator2 _x_3) (Utilities|Select :Index YSizeMode :NewEnumerator0 _y :NewEnumerator1 _y_2 :NewEnumerator2 _y_3) (Utilities|Select :Index ZSizeMode :NewEnumerator0 _z :NewEnumerator1 _z_2 :NewEnumerator2 _z_3))))