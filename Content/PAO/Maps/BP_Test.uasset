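; BP_Test is a test actor that places and sizes a Tube static mesh component from initial location, rotation and size variables.
; The construction script divides InitSize by the mesh's bounding box extents to get its scale, then offsets InitLocation by half the rotated size.
; It stores the result in PrevTransform and applies it as the Tube's relative transform.
; The event graph is empty, and a ComposeTransforms chain is left unused.
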(event EventBeginPlay)

(event Collision|EventActorBeginOverlap
  (params (OtherActor :type Actor%20Object%20Reference)))

(event EventTick
  (params (DeltaSeconds :type Float%20%28single-precision%29)))

(fn ConstructionScript
  (bind _tube (Variables|Default|GetTube))
  (bind _staticmesh (Variables|/Script/Engine.StaticMeshComponent|GetStaticMesh _tube))
  (bind _returnvalue (StaticMesh|GetBoundingBox _staticmesh))
  (LocalVariables|Set_OriginSize (- (.max _returnvalue) (.min _returnvalue)))
  (LocalVariables|Set_InitRotate (Variables|Default|GetInitRotate))
  (LocalVariables|Set_InitScale (/ (Variables|Default|GetInitSize) (LocalVariables|Get_OriginSize)))
  (bind _output_get (LocalVariables|Set_PrevTransform (Math|Transform|MakeTransform (+ (Variables|Default|GetInitLocation) (/ (Math|Vector|RotateVector (Variables|Default|GetInitSize) (Variables|Default|GetInitRotate)) 2)) (Variables|Default|GetInitRotate) (LocalVariables|Get_InitScale))))
  (Transformation|SetRelativeTransform (Variables|Default|GetTube) _output_get false false))